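; Fish NPC actor that tracks how quickly its mesh is turning in yaw.
; BeginPlay stores the mesh's starting world rotation, and each Tick takes the yaw of the previous rotation minus the current one, then saves the current rotation.
; RotAngleDifference eases toward that delta with a fixed-alpha Lerp, giving a smoothed per-frame turn value that is not scaled by delta time.
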(event `self.ReceiveTick`
  (params (DeltaSeconds :type "Float (single-precision)"))
  (bind _returnvalue (`SceneComponent.K2_GetComponentRotation` (`self.Mesh`)))
  (bind (_returnvalue_roll _returnvalue_pitch _returnvalue_yaw) (`KismetMathLibrary.BreakRotator` (`KismetMathLibrary.NormalizedDeltaRotator` (`self.LastRotation`) _returnvalue)))
  ;[1 1 1] FindDeltaRotation
  (set `self.RotAngleDifference` (`KismetMathLibrary.Lerp` (`self.RotAngleDifference`) _returnvalue_yaw 0.1))
  (set `self.LastRotation` _returnvalue))

(event `self.ReceiveBeginPlay`
  ;[1 1 1] FindDeltaRotation
  (set `self.LastRotation` (`SceneComponent.K2_GetComponentRotation` (`self.Mesh`))))

(fn `UserConstructionScript`)