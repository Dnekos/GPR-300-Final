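; Duckweed food actor that fish, either the player character or AI fish, can eat.
; A Sphere trigger sets Skimming on an overlapping Fish-tagged ThirdPersonCharacter_2 or BP_Fish_AI and clears it on exit.
; When a tagged fish touches the Cube, the duckweed plays a sound, spawns a splash particle and destroys itself.
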(event `self.ReceiveActorBeginOverlap`
  (params (OtherActor :type "Actor Object Reference")))

(event `self.Cube.OnComponentBeginOverlap`
  (params (OverlappedComponent :type "PrimitiveComponent Object Reference") (OtherActor :type "Actor Object Reference") (OtherComp :type "PrimitiveComponent Object Reference") (OtherBodyIndex :type Integer) (bFromSweep :type Boolean) (SweepResult :type "HitResult Structure (by ref)"))
  (if (`self.ActorHasTag` OtherActor "Fish")
    (`KismetSystemLibrary.PrintString` "Fish Ate Food" false)
    (`GameplayStatics.PlaySound2D` "/Game/Sounds/fishSwimSound.fishSwimSound" 1.0 1.0 0.0 null null)
    (`GameplayStatics.SpawnEmitterAtLocation` "/Game/Actors/SplashParticle.SplashParticle" (`SceneComponent.K2_GetComponentLocation` (`self.DefaultSceneRoot`)))
    (`self.K2_DestroyActor`)))

(event `self.Sphere.OnComponentBeginOverlap`
  (params (OverlappedComponent :type "PrimitiveComponent Object Reference") (OtherActor :type "Actor Object Reference") (OtherComp :type "PrimitiveComponent Object Reference") (OtherBodyIndex :type Integer) (bFromSweep :type Boolean) (SweepResult :type "HitResult Structure (by ref)"))
  (if (`self.ActorHasTag` OtherActor "Fish")
    (bind _asthird_person_character_2 (cast `/Game/fish/ThirdPersonCharacter_2` OtherActor)
      (:`then`
        (set `/Game/fish/ThirdPersonCharacter_2.Skimming` true _asthird_person_character_2))
      (:`CastFailed`
        (bind _asbp_fish_ai (cast `/Game/Actors/FishNPC/BP_Fish_AI` OtherActor))
        (set `/Game/Actors/FishNPC/BP_Fish_AI.Skimming` true _asbp_fish_ai)))))

(event `self.Sphere.OnComponentEndOverlap`
  (params (OverlappedComponent :type "PrimitiveComponent Object Reference") (OtherActor :type "Actor Object Reference") (OtherComp :type "PrimitiveComponent Object Reference") (OtherBodyIndex :type Integer))
  (if (`self.ActorHasTag` OtherActor "Fish")
    (bind _asthird_person_character_2 (cast `/Game/fish/ThirdPersonCharacter_2` OtherActor)
      (:`then`
        (set `/Game/fish/ThirdPersonCharacter_2.Skimming` false _asthird_person_character_2))
      (:`CastFailed`
        (bind _asbp_fish_ai (cast `/Game/Actors/FishNPC/BP_Fish_AI` OtherActor))
        (set `/Game/Actors/FishNPC/BP_Fish_AI.Skimming` false _asbp_fish_ai)))))

(fn `UserConstructionScript`)